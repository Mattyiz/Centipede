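; Mushroom obstacle actor for a Centipede game that takes hits and awards score when destroyed.
; It starts with three health on BeginPlay, and each Shot call removes one point.
; At zero health it finds the GameManager_BP via GetAllActorsOfClass, adds one to its Score and destroys itself.
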(event EventBeginPlay
  (Variables|Default|SetHealth 3)
  (|CallParentFunction))

(event Collision|EventActorBeginOverlap
  (params (OtherActor :type Actor%20Object%20Reference))
  (|CallParentFunction OtherActor) ; This node is disabled and will not be called.\nDrag off pins to build functionality.
)

(event EventTick
  (params (DeltaSeconds :type Float%20%28single-precision%29))
  (|CallParentFunction DeltaSeconds) ; This node is disabled and will not be called.\nDrag off pins to build functionality.
)

(fn ConstructionScript
  (|CallParentFunction))

(fn Shot
  (bind _output_get (Variables|Default|SetHealth (- (Variables|Default|GetHealth) 1)))
  (if (<= _output_get 0)
    (bind _outactors (Actor|GetAllActorsOfClass "/Game/Centipede/GameManager_BP.GameManager_BP_C"))
    (Variables|/Game/Centipede/GameManager_BP.GameManager_BP_C|SetScore (Utilities|Array|Get(acopy) _outactors) (+ (Variables|/Game/Centipede/GameManager_BP.GameManager_BP_C|GetScore (Utilities|Array|Get(acopy) _outactors)) 1))
    (Actor|DestroyActor)))