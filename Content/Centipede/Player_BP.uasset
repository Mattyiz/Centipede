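; Player Blueprint for a Centipede game: a cube that moves within a bounded rectangle and fires Bullet_BP from BulletSpawn.
; Axis inputs apply bounds-checked per-frame offsets, unscaled by delta time.
; Overlapping any non-mushroom enemy costs a life, starts brief invincibility and resets position, or destroys the cube once lives drop below zero.
; Tick counts down invincibility and awards extra lives from GameManager_BP's score since last life.
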(event OnComponentBeginOverlap(Cube)
  (params (OverlappedComponent :type Primitive%20Component%20Object%20Reference) (OtherActor :type Actor%20Object%20Reference) (OtherComp :type Primitive%20Component%20Object%20Reference) (OtherBodyIndex :type Integer) (bFromSweep :type Boolean) (SweepResult :type Hit%20Result%20Structure%20%28by%20ref%29))
  (Utilities|Casting|CastToEnemyBase_BP OtherActor)
  (Utilities|Casting|CastToMushroom_BP OtherActor
    (:CastFailed
      (if (not (> (Variables|Default|GetInvinicibility) 0.0))
        (Variables|Default|SetInvinicibility 1.0)
        (bind _output_get (Variables|Default|SetLives (- (Variables|Default|GetLives) 1)))
        (if (>= _output_get 0)
          (Transformation|SetWorldLocation (Variables|Default|GetCube) "0.000000,-2000.000000,0.000000" false false)
          (else
            (Components|DestroyComponent (Variables|Default|GetCube))
            (Variables|Default|SetDead true)))))))

(event EventBeginPlay
  (Transformation|SetWorldLocation (Variables|Default|GetCube) "0.000000,-2000.000000,0.000000" false false)
  (Variables|Default|SetDead false)
  (Variables|Default|SetLives 3)
  (bind _outactors (Actor|GetAllActorsOfClass "/Game/Centipede/GameManager_BP.GameManager_BP_C"))
  (Variables|Default|SetGameManager (Utilities|Array|Get(acopy) _outactors)))

(event EventTick
  (params (DeltaSeconds :type Float%20%28single-precision%29))
  (bind _gamemanager (Variables|Default|GetGameManager))
  (if (> (Variables|Default|GetInvinicibility) 0.0)
    (Variables|Default|SetInvinicibility (- (Variables|Default|GetInvinicibility) DeltaSeconds)))
  (if (>= (Variables|/Game/Centipede/GameManager_BP.GameManager_BP_C|GetScoreSinceLife (Variables|Default|GetGameManager)) 12000)
    (Variables|Default|SetLives (+ (Variables|Default|GetLives) 1))
    (Variables|/Game/Centipede/GameManager_BP.GameManager_BP_C|SetScoreSinceLife _gamemanager (- (Variables|/Game/Centipede/GameManager_BP.GameManager_BP_C|GetScoreSinceLife _gamemanager) 12000))))

(event Input|ActionEvents|InputActionShoot
  (params (Key :type Key%20Structure :default "None"))
  (:Pressed
    (if (not (Variables|Default|GetDead))
      (Game|SpawnActorfromClass "/Game/Centipede/Bullet_BP.Bullet_BP_C" (Transformation|GetWorldTransform (Variables|Default|GetBulletSpawn)) "Undefined" "MultiplyWithRoot" 0 0))))

(event Input|AxisEvents|InputAxisMoveHorizontal
  (params (AxisValue :type Float%20%28single-precision%29))
  (bind _cube (Variables|Default|GetCube))
  (bind _movespeed (Variables|Default|GetMoveSpeed))
  (bind _returnvalue (Transformation|GetWorldTransform _cube))
  (bind _returnvalue_2 (* AxisValue _movespeed))
  (bind _returnvalue_3 (+ (.x (.location _returnvalue)) _returnvalue_2))
  (if (not (Variables|Default|GetDead))
    (if (> _returnvalue_3 -3e+03)
      (if (< _returnvalue_3 3e+03)
        (Class|SceneComponent|AddLocalTransform _cube (Math|Transform|MakeTransform (Math|Vector|MakeVector _returnvalue_2 0.0 0.0) "0, 0, 0" "1.000000,1.000000,1.000000") false false)))))

(event Input|AxisEvents|InputAxisMoveVertical
  (params (AxisValue :type Float%20%28single-precision%29))
  (bind _cube (Variables|Default|GetCube))
  (bind _movespeed (Variables|Default|GetMoveSpeed))
  (bind _returnvalue (Transformation|GetWorldTransform _cube))
  (bind _returnvalue_2 (* AxisValue _movespeed))
  (bind _returnvalue_3 (+ (.y (.location _returnvalue)) _returnvalue_2))
  (if (not (Variables|Default|GetDead))
    (if (> _returnvalue_3 -2.5e+03)
      (if (< _returnvalue_3 -1e+03)
        (Class|SceneComponent|AddLocalTransform _cube (Math|Transform|MakeTransform (Math|Vector|MakeVector 0.0 _returnvalue_2 0.0) "0, 0, 0" "1.000000,1.000000,1.000000") false false)))))

(fn ConstructionScript)