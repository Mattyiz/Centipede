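; Game manager for a Centipede-style game that scatters mushrooms at start, runs the centipede and periodically spawns a random spider or flea.
; Tick spawns segments on a short stagger to rebuild a killed centipede, then moves every segment sideways, stepping and reversing those flagged GoingDown.
; NewHead removes a shot segment, promotes its follower to head and reindexes the rest.
; While TimeStopped is set, all this pauses and Score drains until zero.
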(event EventBeginPlay
  (for _index (range 0 100)
    (Game|SpawnActorfromClass "/Game/Centipede/Mushroom_BP.Mushroom_BP_C" (Math|Transform|MakeTransform (Math|Vector|MakeVector (Math|Random|RandomFloatinRange -3e+03 3e+03) (Math|Random|RandomFloatinRange -2.5e+03 2.5e+03) 0.0) "0, 0, 0" "1.000000,1.000000,1.000000") "Undefined" "MultiplyWithRoot" 0 0)))

(event Collision|EventActorBeginOverlap
  (params (OtherActor :type Actor%20Object%20Reference)))

(event EventTick
  (params (DeltaSeconds :type Float%20%28single-precision%29))
  (if (Variables|Default|GetTimeStopped)
    (bind _output_get (Variables|Default|SetTimeStopTimer (- (Variables|Default|GetTimeStopTimer) DeltaSeconds)))
    (if (> _output_get 0.0)
      _
      (else
        (Variables|Default|SetTimeStopTimer 0.5)
        (Variables|Default|SetScore (- (Variables|Default|GetScore) 50))))
    (if (<= (Variables|Default|GetScore) 0)
      (Variables|Default|SetTimeStopped false)
      (Variables|Default|SetScore 0))
    (else
      (Variables|Default|SetTimeStopTimer 0.5)
      (Variables|Default|SetSpawnTimer (- (Variables|Default|GetSpawnTimer) DeltaSeconds))
      (Variables|Default|SetExtraSpawnTimer (- (Variables|Default|GetExtraSpawnTimer) DeltaSeconds))
      (if (Variables|Default|GetCentipedeKilled) ; Does there need to be a new centipede?
        (if (< (Utilities|Array|Length (Variables|Default|GetCentipede)) 12) ; Is the centipede long enough
          (if (<= (Variables|Default|GetSpawnTimer) 0.0) ; Don't spawn on each other
            (CallFunction|SpawnCentipede)
            (Variables|Default|SetSpawnTimer 0.12))
          (else
            (Variables|Default|SetCentipedeKilled false))))
      (CallFunction|MoveCentipede)
      (if (<= (Variables|Default|GetExtraSpawnTimer) 0.0)
        (CallFunction|SpawnOthers)
        (Variables|Default|SetExtraSpawnTimer 9.0)))))

(fn ConstructionScript)

(fn NewHead
  (params (ShotSegment :type Integer))
  (bind _centipede (Variables|Default|GetCentipede))
  (bind _centipede_2 (Variables|Default|GetCentipede))
  (bind _output (Utilities|Array|Get(acopy) _centipede ShotSegment))
  (Utilities|Array|RemoveIndex _centipede_2 ShotSegment)
  (if (<= (Utilities|Array|Length _centipede_2) 0)
    (Variables|Default|SetCentipedeKilled true)
    (elif (Utilities|Array|IsValidIndex _centipede ShotSegment)
      (if (Utilities|IsValid _output)
        (Default|PromotetoHead _output)
        (for (_array_element _array_index) (Variables|Default|GetCentipede)
          (if (Utilities|IsValid _array_element)
            (if (> (Variables|/Game/Centipede/CentipedeSegment_BP.CentipedeSegment_BP_C|GetSegment _array_element) _array_index)
              (Variables|/Game/Centipede/CentipedeSegment_BP.CentipedeSegment_BP_C|SetSegment _array_element (- (Variables|/Game/Centipede/CentipedeSegment_BP.CentipedeSegment_BP_C|GetSegment _array_element) 1)))))))))

(fn SpawnCentipede
  (bind _centipede (Variables|Default|GetCentipede))
  (bind _returnvalue (Game|SpawnActorfromClass "/Game/Centipede/CentipedeSegment_BP.CentipedeSegment_BP_C" (Math|Transform|MakeTransform "0.000000,2500.000000,0.000000" "0, 0, 0" "1.000000,1.000000,1.000000") "Undefined" "MultiplyWithRoot" 0 0))
  (bind _returnvalue_2 (Utilities|Array|Add _centipede _returnvalue))
  (Variables|/Game/Centipede/CentipedeSegment_BP.CentipedeSegment_BP_C|SetSegment (Utilities|Array|Get(acopy) _centipede _returnvalue_2) _returnvalue_2)
  (if (<= _returnvalue_2 0)
    (Default|PromotetoHead (Utilities|Array|Get(acopy) _centipede _returnvalue_2))))

(fn MoveCentipede
  (for (_ _array_index) (Variables|Default|GetCentipede)
    (if (Utilities|IsValid (Utilities|Array|Get(acopy) (Variables|Default|GetCentipede) _array_index))
      (if (Variables|/Game/Centipede/CentipedeSegment_BP.CentipedeSegment_BP_C|GetGoingDown (Utilities|Array|Get(acopy) (Variables|Default|GetCentipede) _array_index))
        (Transformation|AddLocalOffset (Variables|/Script/Engine.Actor|GetRootComponent (Utilities|Array|Get(acopy) (Variables|Default|GetCentipede) _array_index)) (Math|Vector|MakeVector 0.0 (Math|Conversions|ToFloat(Integer) (* (Variables|/Game/Centipede/CentipedeSegment_BP.CentipedeSegment_BP_C|GetYDirection (Utilities|Array|Get(acopy) (Variables|Default|GetCentipede) _array_index)) 100)) 0.0) false false)
        (Variables|/Game/Centipede/CentipedeSegment_BP.CentipedeSegment_BP_C|SetXDirection (Utilities|Array|Get(acopy) (Variables|Default|GetCentipede) _array_index) (* (Variables|/Game/Centipede/CentipedeSegment_BP.CentipedeSegment_BP_C|GetXDirection (Utilities|Array|Get(acopy) (Variables|Default|GetCentipede) _array_index)) -1))
        (Variables|/Game/Centipede/CentipedeSegment_BP.CentipedeSegment_BP_C|SetGoingDown (Utilities|Array|Get(acopy) (Variables|Default|GetCentipede) _array_index) false))
      (Transformation|SetWorldLocation (Variables|/Script/Engine.Actor|GetRootComponent (Utilities|Array|Get(acopy) (Variables|Default|GetCentipede) _array_index)) (Math|Vector|MakeVector (+ (.x (Transformation|GetWorldLocation (Variables|/Script/Engine.Actor|GetRootComponent (Utilities|Array|Get(acopy) (Variables|Default|GetCentipede) _array_index)))) (* (Variables|/Game/Centipede/CentipedeSegment_BP.CentipedeSegment_BP_C|GetXDirection (Utilities|Array|Get(acopy) (Variables|Default|GetCentipede) _array_index)) 7)) (.y (Transformation|GetWorldLocation (Variables|/Script/Engine.Actor|GetRootComponent (Utilities|Array|Get(acopy) (Variables|Default|GetCentipede) _array_index)))) (.z (Transformation|GetWorldLocation (Variables|/Script/Engine.Actor|GetRootComponent (Utilities|Array|Get(acopy) (Variables|Default|GetCentipede) _array_index))))) false false))))

(fn SpawnOthers
  (switch int (Math|Random|RandomInteger 2)
    (:0
      (bind _output_get (LocalVariables|SetSpawnX (Math|Random|RandomIntegerinRange -1 1)))
      (if (== _output_get 0)
        (LocalVariables|SetSpawnX 1))
      (bind _output_get_2 (LocalVariables|SetSpawnX (* (LocalVariables|GetSpawnX) 3000)))
      (Game|SpawnActorfromClass "/Game/Centipede/Spider_BP.Spider_BP_C" (Math|Transform|MakeTransform (Math|Vector|MakeVector (Math|Conversions|ToFloat(Integer) _output_get_2) (Math|Random|RandomFloatinRange -1e+03 -2e+03) 0.0) "0, 0, 0" "1.000000,1.000000,1.000000") "Undefined" "MultiplyWithRoot" 0 0))
    (:1
      (Game|SpawnActorfromClass "/Game/Centipede/Flea_BP.Flea_BP_C" (Math|Transform|MakeTransform (Math|Vector|MakeVector (Math|Random|RandomFloatinRange -2.6e+03 2.6e+03) 2.5e+03 0.0) "0, 0, 0" "1.000000,1.000000,1.000000") "Undefined" "MultiplyWithRoot" 0 0))))