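; Bullet_BP is the projectile in the Centipede game, damaging enemies on contact.
; Each tick it moves its Sphere along +Y at a fixed, frame-rate-dependent step and destroys itself past a Y limit if nothing was hit.
; On overlap with an EnemyBase_BP it calls that enemy's Shot, sets Hit and destroys itself, ignoring all other actors.
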(event OnComponentBeginOverlap(Sphere)
  (params (OverlappedComponent :type Primitive%20Component%20Object%20Reference) (OtherActor :type Actor%20Object%20Reference) (OtherComp :type Primitive%20Component%20Object%20Reference) (OtherBodyIndex :type Integer) (bFromSweep :type Boolean) (SweepResult :type Hit%20Result%20Structure%20%28by%20ref%29))
  (bind _asenemy_base_bp (Utilities|Casting|CastToEnemyBase_BP OtherActor))
  (Default|Shot _asenemy_base_bp)
  (Variables|Default|SetHit true)
  (Actor|DestroyActor))

(event EventBeginPlay)

(event Collision|EventActorBeginOverlap
  (params (OtherActor :type Actor%20Object%20Reference)))

(event EventTick
  (params (DeltaSeconds :type Float%20%28single-precision%29))
  (bind _sphere (Variables|Default|GetSphere))
  (Transformation|AddWorldOffset _sphere "0.000000,25.000000,0.000000" false false)
  (if (not (Variables|Default|GetHit))
    (if (> (.y (Transformation|GetWorldLocation _sphere)) 2.8e+03)
      (Actor|DestroyActor))))

(fn ConstructionScript)