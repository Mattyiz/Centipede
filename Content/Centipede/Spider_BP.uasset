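; Spider enemy for a Centipede-style game that roams the play field and destroys any mushroom it overlaps.
; Tick moves its Sphere by per-frame offsets not scaled by delta time, bouncing off fixed X and Y limits.
; A repeating timer flips vertical direction and occasionally re-randomizes horizontal speed.
; Shot adds points to both score counters on the GameManager found at BeginPlay, then destroys the spider.
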(event EventBeginPlay
  (bind _outactors (Actor|GetAllActorsOfClass "/Game/Centipede/GameManager_BP.GameManager_BP_C"))
  (Variables|Default|SetGameManager (Utilities|Array|Get(acopy) _outactors))
  (Variables|Default|SetXSpeed (Math|Random|RandomFloatinRange 2.0 1e+01))
  (Variables|Default|SetChange%20Timer 3.0))

(event Collision|EventActorBeginOverlap
  (params (OtherActor :type Actor%20Object%20Reference))
  (Utilities|Casting|CastToMushroom_BP OtherActor)
  (Actor|DestroyActor OtherActor))

(event EventTick
  (params (DeltaSeconds :type Float%20%28single-precision%29))
  (Variables|Default|SetChange%20Timer (- (Variables|Default|GetChange%20Timer) DeltaSeconds))
  (if (<= (Variables|Default|GetChange%20Timer) 0.0)
    (Variables|Default|SetChange%20Timer 3.0)
    (Variables|Default|SetYSpeed (* (Variables|Default|GetYSpeed) -1.0))
    (if (<= (Math|Random|RandomIntegerinRange 0 10) 2)
      (Variables|Default|SetXSpeed (Math|Random|RandomFloatinRange -1e+01 1e+01))))
  (CallFunction|Move))

(fn ConstructionScript
  (|CallParentFunction))

(fn Shot
  (bind _gamemanager (Variables|Default|GetGameManager))
  (Variables|/Game/Centipede/GameManager_BP.GameManager_BP_C|SetScore _gamemanager (+ (Variables|/Game/Centipede/GameManager_BP.GameManager_BP_C|GetScore _gamemanager) 300))
  (Variables|/Game/Centipede/GameManager_BP.GameManager_BP_C|SetScoreSinceLife (Variables|Default|GetGameManager) (+ (Variables|/Game/Centipede/GameManager_BP.GameManager_BP_C|GetScoreSinceLife _gamemanager) 300))
  (Actor|DestroyActor))

(fn Move
  (bind _sphere (Variables|Default|GetSphere))
  (bind _sphere_2 (Variables|Default|GetSphere))
  (bind _returnvalue (Transformation|GetWorldLocation _sphere))
  (bind _returnvalue_2 (Transformation|GetWorldLocation _sphere_2))
  (Transformation|AddWorldOffset (Variables|Default|GetSphere) (Math|Vector|MakeVector (Variables|Default|GetXSpeed) (Variables|Default|GetYSpeed) 0.0) false false)
  (if (and (or (>= (.y _returnvalue_2) 0.0) (<= (.y _returnvalue_2) -2.5e+03)) (Utilities|IsValid (Variables|Default|GetSphere)))
    (bind _output_get (Variables|Default|SetYSpeed (* (Variables|Default|GetYSpeed) -1.0)))
    (Transformation|AddWorldOffset (Variables|Default|GetSphere) (Math|Vector|MakeVector 0.0 _output_get 0.0) false false))
  (if (and (or (>= (.x _returnvalue) 3e+03) (<= (.x _returnvalue) -3e+03)) (Utilities|IsValid (Variables|Default|GetSphere)))
    (bind _output_get_2 (Variables|Default|SetXSpeed (* (Variables|Default|GetXSpeed) -1.0)))
    (Transformation|AddWorldOffset (Variables|Default|GetSphere) (Math|Vector|MakeVector _output_get_2 0.0 0.0) false false)))