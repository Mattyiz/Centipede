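; CentipedeSegment_BP is one centipede segment that scores when shot, with a head worth more than a body segment.
; Shot adds to the GameManager's score counters, spawns a mushroom in the segment's place, calls NewHead with its Segment value, then destroys the segment.
; Mushroom overlaps and X-axis bounds set GoingDown, but the step-down and direction-flip nodes are disconnected, so this graph never moves the segment.
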(event EventBeginPlay
  (bind _outactors (Actor|GetAllActorsOfClass "/Game/Centipede/GameManager_BP.GameManager_BP_C"))
  (Variables|Default|SetGameManager (Utilities|Array|Get(acopy) _outactors)))

(event Collision|EventActorBeginOverlap
  (params (OtherActor :type Actor%20Object%20Reference))
  (Utilities|Casting|CastToMushroom_BP OtherActor)
  (Variables|Default|SetGoingDown true))

(event EventTick
  (params (DeltaSeconds :type Float%20%28single-precision%29))
  (bind _sphere (Variables|Default|GetSphere))
  (bind _returnvalue (Transformation|GetWorldLocation _sphere))
  (if (or (>= (.x _returnvalue) 3e+03) (<= (.x _returnvalue) -3e+03))
    (Variables|Default|SetGoingDown true)))

(fn ConstructionScript
  (|CallParentFunction))

(fn Shot
  (bind _gamemanager (Variables|Default|GetGameManager))
  (bind _gamemanager_2 (Variables|Default|GetGameManager))
  (if (Variables|Default|GetIsHead)
    (Variables|/Game/Centipede/GameManager_BP.GameManager_BP_C|SetScore _gamemanager (+ (Variables|/Game/Centipede/GameManager_BP.GameManager_BP_C|GetScore _gamemanager) 100))
    (Variables|/Game/Centipede/GameManager_BP.GameManager_BP_C|SetScoreSinceLife (Variables|Default|GetGameManager) (+ (Variables|/Game/Centipede/GameManager_BP.GameManager_BP_C|GetScoreSinceLife _gamemanager) 100))
    (else
      (Variables|/Game/Centipede/GameManager_BP.GameManager_BP_C|SetScore _gamemanager_2 (+ (Variables|/Game/Centipede/GameManager_BP.GameManager_BP_C|GetScore _gamemanager_2) 10))
      (Variables|/Game/Centipede/GameManager_BP.GameManager_BP_C|SetScoreSinceLife (Variables|Default|GetGameManager) (+ (Variables|/Game/Centipede/GameManager_BP.GameManager_BP_C|GetScoreSinceLife _gamemanager_2) 10))))
  (Game|SpawnActorfromClass "/Game/Centipede/Mushroom_BP.Mushroom_BP_C" (Math|Transform|MakeTransform (Transformation|GetWorldLocation (Variables|Default|GetSphere)) "0, 0, 0" "1.000000,1.000000,1.000000") "Undefined" "MultiplyWithRoot" 0 0)
  (Default|NewHead (Variables|Default|GetGameManager) (Variables|Default|GetSegment))
  (Actor|DestroyActor))