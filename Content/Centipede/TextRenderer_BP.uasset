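; TextRenderer_BP is the on-screen text display for the Centipede game, showing the current score and remaining lives.
; On BeginPlay it finds and caches the first GameManager_BP and Player_BP actors in the level.
; It writes their Score and Lives values into its Score and Lives text components, then refreshes both every Tick by polling rather than using events.
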(event EventBeginPlay
  (bind _outactors (Actor|GetAllActorsOfClass "/Game/Centipede/GameManager_BP.GameManager_BP_C"))
  (bind _output_get (Variables|Default|SetGameManager (Utilities|Array|Get(acopy) _outactors)))
  (Rendering|Components|TextRender|SetText (Variables|Default|GetScore) (Utilities|Text|ToText(Integer) (Variables|/Game/Centipede/GameManager_BP.GameManager_BP_C|GetScore _output_get)))
  (bind _outactors_2 (Actor|GetAllActorsOfClass "/Game/Centipede/Player_BP.Player_BP_C"))
  (Variables|Default|SetPlayer (Utilities|Array|Get(acopy) _outactors_2))
  (Rendering|Components|TextRender|SetText (Variables|Default|GetLives) (Utilities|Text|ToText(Integer) (Variables|/Game/Centipede/Player_BP.Player_BP_C|GetLives (Utilities|Array|Get(acopy) _outactors_2)))))

(event Collision|EventActorBeginOverlap
  (params (OtherActor :type Actor%20Object%20Reference)))

(event EventTick
  (params (DeltaSeconds :type Float%20%28single-precision%29))
  (Rendering|Components|TextRender|SetText (Variables|Default|GetScore) (Utilities|Text|ToText(Integer) (Variables|/Game/Centipede/GameManager_BP.GameManager_BP_C|GetScore (Variables|Default|GetGameManager))))
  (Rendering|Components|TextRender|SetText (Variables|Default|GetLives) (Utilities|Text|ToText(Integer) (Variables|/Game/Centipede/Player_BP.Player_BP_C|GetLives (Variables|Default|GetPlayer)))))

(fn ConstructionScript)