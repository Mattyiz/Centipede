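; Flea enemy for a Centipede-style game that moves along negative Y and leaves mushrooms behind it.
; Tick shifts the Sphere component by YSpeed each frame, without delta-time scaling, and spawns Mushroom_BP at its location on a randomized short timer.
; Shot decrements HP, and the second hit adds points to both GameManager score counters and destroys the actor.
; Overlap events only set an Overlapping flag.
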(event EventBeginPlay
  (bind _outactors (Actor|GetAllActorsOfClass "/Game/Centipede/GameManager_BP.GameManager_BP_C"))
  (Variables|Default|SetGameManager (Utilities|Array|Get(acopy) _outactors))
  (Variables|Default|SetHP 2))

(event EventTick
  (params (DeltaSeconds :type Float%20%28single-precision%29))
  (bind _sphere (Variables|Default|GetSphere))
  (bind _returnvalue (Transformation|GetWorldLocation _sphere))
  (Variables|Default|SetMushroomTimer (- (Variables|Default|GetMushroomTimer) DeltaSeconds))
  (Transformation|SetWorldLocation (Variables|Default|GetSphere) (Math|Vector|MakeVector (.x _returnvalue) (- (.y _returnvalue) (Variables|Default|GetYSpeed)) 0.0) false false)
  (if (<= (Variables|Default|GetMushroomTimer) 0.0)
    (Variables|Default|SetMushroomTimer (Math|Random|RandomFloatinRange 0.1 0.5))
    (Game|SpawnActorfromClass "/Game/Centipede/Mushroom_BP.Mushroom_BP_C" (Math|Transform|MakeTransform (Transformation|GetWorldLocation (Variables|Default|GetSphere)) "0, 0, 0" "1.000000,1.000000,1.000000") "Undefined" "MultiplyWithRoot" 0 0)))

(event Collision|EventActorBeginOverlap
  (params (OtherActor :type Actor%20Object%20Reference))
  (Variables|Default|SetOverlapping true))

(event Collision|EventActorEndOverlap
  (params (OtherActor :type Actor%20Object%20Reference))
  (Variables|Default|SetOverlapping false))

(fn ConstructionScript
  (|CallParentFunction))

(fn Shot
  (bind _gamemanager (Variables|Default|GetGameManager))
  (bind _output_get (Variables|Default|SetHP (- (Variables|Default|GetHP) 1)))
  (if (<= _output_get 0)
    (Variables|/Game/Centipede/GameManager_BP.GameManager_BP_C|SetScore _gamemanager (+ (Variables|/Game/Centipede/GameManager_BP.GameManager_BP_C|GetScore _gamemanager) 200))
    (Variables|/Game/Centipede/GameManager_BP.GameManager_BP_C|SetScoreSinceLife (Variables|Default|GetGameManager) (+ (Variables|/Game/Centipede/GameManager_BP.GameManager_BP_C|GetScoreSinceLife _gamemanager) 200))
    (Actor|DestroyActor)))